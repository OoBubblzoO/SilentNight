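; BP_Note is a readable note actor that toggles an on-screen note when interacted with.
; The Interact event checks the IsReading flag: when false, it plays a pickup sound, creates a WB_Note widget, stores it and adds it to the viewport.
; The next interaction clears the flag and removes the stored widget from the screen.
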(event `/Game/Blueprints/BPI_Interaction.Interact`
  (if (not (`self.Is Reading`))
    (set `self.Is Reading` true)
    (`GameplayStatics.PlaySound2D` "/Game/Audio/NotePickup.NotePickup" 1.0 1.0 0.0 null null)
    (bind _returnvalue (`|CreateWidget` "/Game/UI/WB_Note.WB_Note_C"))
    (bind _output_get (set `self.Notes REF` _returnvalue))
    (`UserWidget.AddToViewport` _output_get 0)
    (else
      (set `self.Is Reading` false)
      (`Widget.RemoveFromParent` (`self.Notes REF`)))))

(fn `UserConstructionScript`)