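; BP_Lightswitch is an interactable switch that toggles the lights linked to it by a matching LightIndex.
; On BeginPlay it caches every BP_Light in the level.
; Its trigger enables input and opens a Gate while the first-person character overlaps, reversing both on exit.
; Interact passes through that Gate, then sends ToggleLightsMessage to each matching light and plays a 2D switch sound.
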(event `self.ReceiveBeginPlay`
  ;[1 1 1] Adding all the lights into an array at the beginning of the game
  (bind _outactors (`GameplayStatics.GetAllActorsOfClass` "/Game/Blueprints/BP_Light.BP_Light_C"))
  (for _array_element _outactors
    (`KismetArrayLibrary.Array_Add` (`self.Light Array`) _array_element)))

(event `/Game/Blueprints/BPI_Interaction.Interact`
  (`/Engine/EditorBlueprintResources/StandardMacros.Gate` false :!label _label
    (:`Exit`
      ;[1 1 1] get light index from light loop and light switch
      (for _array_element (`self.Light Array`)
        (if (== (`/Game/Blueprints/BP_Light.Light Index` _array_element) (`self.Light Index`))
          (message `/Game/Blueprints/BPI_Lights.Toggle Lights` _array_element)
          (`GameplayStatics.PlaySound2D` "/Game/Audio/Lightswitchsound.Lightswitchsound" 1.0 1.0 0.0 null null))))))

(event `self.Trigger.OnComponentBeginOverlap`
  (params (OverlappedComponent :type "PrimitiveComponent Object Reference") (OtherActor :type "Actor Object Reference") (OtherComp :type "PrimitiveComponent Object Reference") (OtherBodyIndex :type Integer) (bFromSweep :type Boolean) (SweepResult :type "HitResult Structure (by ref)"))
  (cast `/Game/ThirdPerson/Blueprints/BP_FirstPersonCharacter` OtherActor)
  (`self.EnableInput` (`GameplayStatics.GetPlayerController` 0))
  (goto _label :!via `Open`))

(event `self.Trigger.OnComponentEndOverlap`
  (params (OverlappedComponent :type "PrimitiveComponent Object Reference") (OtherActor :type "Actor Object Reference") (OtherComp :type "PrimitiveComponent Object Reference") (OtherBodyIndex :type Integer))
  (cast `/Game/ThirdPerson/Blueprints/BP_FirstPersonCharacter` OtherActor)
  (`self.DisableInput` (`GameplayStatics.GetPlayerController` 0))
  (goto _label :!via `Close`))

(fn `UserConstructionScript`)