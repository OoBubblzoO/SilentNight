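; Door Blueprint that stays locked until its key is picked up.
; PickupKey sets the HasKey flag; Interact without it plays a locked sound.
; With the key, a FlipFlop on Interact alternates between playing the door timeline with an opening sound and silently reversing it.
; The timeline's track drives a Lerp on the mesh's relative yaw to swing the door a quarter turn.
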(event `/Game/Blueprints/BPI_Interaction.Interact`
  ;[1 1 1] Open the door only if the player has the key to it
  (if (`self.HasKey?`)
    (`/Engine/EditorBlueprintResources/StandardMacros.FlipFlop`
      (:`A`
        (`GameplayStatics.PlaySound2D` "/Game/Audio/DoorNoiseOpen.DoorNoiseOpen" 1.0 1.0 0.0 null null)
        (bind (_direction _door_track) (`Timeline|Door Timeline` :!label _label)
          (:`Update`
            (`SceneComponent.K2_SetRelativeRotation` (`self.StaticMesh`) (`KismetMathLibrary.MakeRotator` 0.0 0.0 (`KismetMathLibrary.Lerp` 0.0 90.0 _door_track)) false false))))
      (:`B`
        (goto _label :!via `Reverse`)))
    (else
      (set `self.HasKey?` false)
      (`GameplayStatics.PlaySound2D` "/Game/Audio/DoorLocked.DoorLocked" 1.0 1.0 0.0 null null))))

(event `/Game/Blueprints/BPI_Door.Pickup Key`
  ;[1 1 1] Open the door only if the player has the key to it
  (set `self.HasKey?` true))

(fn `UserConstructionScript`)